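; AI controller for the Hunter that runs BT_Hunter on BeginPlay and feeds its blackboard from AI perception.
; Sensed stimuli tagged "kazoo" store a last-heard location; other stimuli set a BP_Duck as target, or clear it if that duck is hidden.
; Any unsuccessfully sensed update clears the target, whatever its source.
; Helpers expose the current target and clear the last-heard location.
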(event OnTargetPerceptionUpdated(AIPerception)
  (params (Actor :type Actor%20Object%20Reference) (Stimulus :type AI%20Stimulus%20Structure))
  (bind _returnvalue (AI|GetBlackboard 0))
  (bind _bb_targetactor (Variables|Default|GetBB_TargetActor))
  (if (.bsuccessfullysensed Stimulus)
    (if (== (.tag Stimulus) "kazoo")
      (AI|Components|Blackboard|SetValueasVector _returnvalue (Variables|Default|GetBB_LastHeardLocation) (.stimuluslocation Stimulus))
      (else
        (bind _asbp_duck (Utilities|Casting|CastToBP_Duck Actor))
        (if (Variables|/Game/BLUEPRINT/DUCK/BP_Duck.BP_Duck_C|GetbIsHidden _asbp_duck)
          (AI|Components|Blackboard|ClearValue (AI|GetBlackboard 0) (Variables|Default|GetBB_TargetActor))
          (else
            (AI|Components|Blackboard|SetValueasObject _returnvalue _bb_targetactor Actor)))))
    (else
      (AI|Components|Blackboard|ClearValue _returnvalue _bb_targetactor))))

(event Custom|ClearLastHeardLocation
  (AI|Components|Blackboard|ClearValue (AI|GetBlackboard 0) (Variables|Default|GetBB_LastHeardLocation)))

(event EventBeginPlay
  (AI|RunBehaviorTree "/Game/BLUEPRINT/HUNTER/BT_Hunter.BT_Hunter"))

(event EventTick
  (params (DeltaSeconds :type Float%20%28single-precision%29)))

(fn ConstructionScript)

(fn GetCurrentTarget
  (return (AI|Components|Blackboard|GetValueasObject (AI|GetBlackboard 0) (Variables|Default|GetBB_TargetActor))))