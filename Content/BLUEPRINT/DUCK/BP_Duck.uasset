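; Player duck pawn that is hunted by a BP_Hunter it spawns on authority, with Enhanced Input movement and look.
; Its kazoo emits an AI noise event and makes nearby hunters flee, earning berries, while being killed adds a roast and respawns it at a random PlayerStart.
; A third berry or roast updates BP_GameMode and returns to the main menu.
; It also drives WBP_HUD counters, timer, hidden status and underwater overlay.
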(event Custom|RespawnPlayer
  (CallFunction|AddRoasts)
  (if (Variables|Default|GetbIsDone)
    (bind _outactors (Actor|GetAllActorsOfClass "/Script/Engine.PlayerStart"))
    (Transformation|SetActorLocation (Transformation|GetActorLocation (Utilities|Array|Get(acopy) _outactors (Math|Random|RandomIntegerinRange 0 (- (Utilities|Array|Length _outactors) 1)))) false false)
    (else
      (Utilities|FlowControl|Delay 5.0)
      (Game|OpenLevel(byName) "L_MainMenu"))))

(event Custom|Kill
  (Input|DisableInput 0)
  (Rendering|SetActorHiddenInGame true)
  (Utilities|FlowControl|Delay 5.0)
  (CallFunction|RespawnPlayer)
  (Rendering|SetActorHiddenInGame false)
  (Input|EnableInput 0))

(event Input|EnhancedActionEvents|EnhancedInputActionIA_Kazoo
  (params (ActionValue :type Boolean) (ElapsedSeconds :type Float%20%28double-precision%29) (TriggeredSeconds :type Float%20%28double-precision%29) (InputAction :type Input%20Action%20Object%20Reference :default "/Game/InputAction/IA_Kazoo.IA_Kazoo"))
  (:Started
    (Audio|PlaySound2D "/Game/BLUEPRINT/DUCK/kazoo.kazoo" 1.0 1.0 0.0 0 0)
    (Class|AISenseHearing|ReportNoiseEvent (Transformation|GetActorLocation) 1.0 self 0.0 "kazoo")
    (bind _outactors (Actor|GetAllActorsOfClass "/Game/BLUEPRINT/HUNTER/BP_Hunter.BP_Hunter_C"))
    (for _array_element _outactors
      (if (<= (Math|Vector|Distance(Vector) (Transformation|GetActorLocation _array_element) (Transformation|GetActorLocation)) 3e+02)
        (Default|StartFlee _array_element)
        (if (Variables|/Game/BLUEPRINT/HUNTER/BP_Hunter.BP_Hunter_C|Getb_CanEarn _array_element)
          (CallFunction|AddBerries)
          (Variables|/Game/BLUEPRINT/HUNTER/BP_Hunter.BP_Hunter_C|Setb_CanEarn _array_element false)
          (if (not (Variables|Default|GetbIsDone))
            (Utilities|FlowControl|Delay 5.0)
            (Game|OpenLevel(byName) "L_MainMenu")))))))

(event Input|EnhancedActionEvents|EnhancedInputActionIA_Right
  (params (ActionValue :type Float%20%28double-precision%29) (ElapsedSeconds :type Float%20%28double-precision%29) (TriggeredSeconds :type Float%20%28double-precision%29) (InputAction :type Input%20Action%20Object%20Reference :default "/Game/InputAction/IA_Right.IA_Right"))
  (Pawn|Input|AddMovementInput (Math|Vector|GetRightVector (Math|Rotator|MakeRotator 0.0 0.0 (.yaw (Pawn|GetControlRotation :!class /Script/Engine.Pawn)))) ActionValue false))

(event Input|EnhancedActionEvents|EnhancedInputActionIA_Forward
  (params (ActionValue :type Float%20%28double-precision%29) (ElapsedSeconds :type Float%20%28double-precision%29) (TriggeredSeconds :type Float%20%28double-precision%29) (InputAction :type Input%20Action%20Object%20Reference :default "/Game/InputAction/IA_Forward.IA_Forward"))
  (Pawn|Input|AddMovementInput (Math|Vector|GetForwardVector (Math|Rotator|MakeRotator 0.0 0.0 (.yaw (Pawn|GetControlRotation :!class /Script/Engine.Pawn)))) ActionValue false))

(event Input|EnhancedActionEvents|EnhancedInputActionIA_Look
  (params (ActionValue :type Vector%202D%20Structure) (ElapsedSeconds :type Float%20%28double-precision%29) (TriggeredSeconds :type Float%20%28double-precision%29) (InputAction :type Input%20Action%20Object%20Reference :default "/Game/InputAction/IA_Look.IA_Look"))
  (Pawn|Input|AddControllerYawInput (.x ActionValue))
  (Pawn|Input|AddControllerPitchInput (.y ActionValue)))

(event EventBeginPlay
  (Utilities|FlowControl|Sequence
    (:then_0
      (CallFunction|CreateHUD))
    (:then_1
      (CallFunction|SpawnHunter))))

(event Collision|EventActorBeginOverlap
  (params (OtherActor :type Actor%20Object%20Reference)))

(event EventTick
  (params (DeltaSeconds :type Float%20%28single-precision%29))
  (CallFunction|UpdateTime))

(fn ConstructionScript)

(fn CreateHUD
  (if (Pawn|IsLocallyControlled)
    (bind _returnvalue (Game|GetCurrentLevelName true))
    (if (Utilities|Enum|Equal(Enum) _returnvalue "LVL_MAPTEST")
      (bind _returnvalue_2 (UserInterface|CreateWidget "/Game/BLUEPRINT/DUCK/WBP_HUD.WBP_HUD_C"))
      (bind _output_get (Variables|Default|SetHUD _returnvalue_2))
      (UserInterface|Viewport|AddtoViewport _output_get 0))))

(fn AddBerries
  (Utilities|IsValid (Variables|Default|GetHUD)
    (:Is%20Valid
      (if (== (Variables|Default|GetBerries) 0)
        (Widget|SetVisibility (Variables|/Game/BLUEPRINT/DUCK/WBP_HUD.WBP_HUD_C|GetB1 (Variables|Default|GetHUD)) "Visible")
        (Variables|Default|SetBerries 1)
        (elif (== (Variables|Default|GetBerries) 1)
          (Widget|SetVisibility (Variables|/Game/BLUEPRINT/DUCK/WBP_HUD.WBP_HUD_C|GetB2 (Variables|Default|GetHUD)) "Visible")
          (Variables|Default|SetBerries 2)
          (elif (== (Variables|Default|GetBerries) 2)
            (Widget|SetVisibility (Variables|/Game/BLUEPRINT/DUCK/WBP_HUD.WBP_HUD_C|GetB3 (Variables|Default|GetHUD)) "Visible")
            (bind _asbp_game_mode (Utilities|Casting|CastToBP_GameMode (Game|GetGameMode)))
            (Default|UpdateState _asbp_game_mode "NewEnumerator0")
            (Variables|Default|SetbIsDone false)))))))

(fn AddRoasts
  (Utilities|IsValid (Variables|Default|GetHUD)
    (:Is%20Valid
      (if (== (Variables|Default|GetRoast) 0)
        (Widget|SetVisibility (Variables|/Game/BLUEPRINT/DUCK/WBP_HUD.WBP_HUD_C|GetR1 (Variables|Default|GetHUD)) "Visible")
        (Variables|Default|SetRoast 1)
        (elif (== (Variables|Default|GetRoast) 1)
          (Widget|SetVisibility (Variables|/Game/BLUEPRINT/DUCK/WBP_HUD.WBP_HUD_C|GetR2 (Variables|Default|GetHUD)) "Visible")
          (Variables|Default|SetRoast 2)
          (elif (== (Variables|Default|GetRoast) 2)
            (Widget|SetVisibility (Variables|/Game/BLUEPRINT/DUCK/WBP_HUD.WBP_HUD_C|GetR3 (Variables|Default|GetHUD)) "Visible")
            (bind _asbp_game_mode (Utilities|Casting|CastToBP_GameMode (Game|GetGameMode)))
            (Default|UpdateState _asbp_game_mode "NewEnumerator1")
            (Variables|Default|SetbIsDone false)))))))

(fn ChangeHidden
  (Utilities|IsValid (Variables|Default|GetHUD)
    (:Is%20Valid
      (Rendering|Components|TextRender|SetText (Variables|/Game/BLUEPRINT/DUCK/WBP_HUD.WBP_HUD_C|GetVISIBILE (Variables|Default|GetHUD)) "HIDDEN")
      (Variables|Default|SetbIsHidden true))))

(fn ChangeVisible
  (Utilities|IsValid (Variables|Default|GetHUD)
    (:Is%20Valid
      (Rendering|Components|TextRender|SetText (Variables|/Game/BLUEPRINT/DUCK/WBP_HUD.WBP_HUD_C|GetVISIBILE (Variables|Default|GetHUD)) "VISIBLE")
      (Variables|Default|SetbIsHidden false))))

(fn InWater
  (Utilities|IsValid (Variables|Default|GetHUD)
    (:Is%20Valid
      (Widget|SetVisibility (Variables|/Game/BLUEPRINT/DUCK/WBP_HUD.WBP_HUD_C|Getunderwater (Variables|Default|GetHUD)) "Visible"))))

(fn OutWater
  (Utilities|IsValid (Variables|Default|GetHUD)
    (:Is%20Valid
      (Widget|SetVisibility (Variables|/Game/BLUEPRINT/DUCK/WBP_HUD.WBP_HUD_C|Getunderwater (Variables|Default|GetHUD)) "Hidden"))))

(fn SpawnHunter
  (Networking|SwitchHasAuthority
    (:Authority
      (Game|SpawnActorfromClass "/Game/BLUEPRINT/HUNTER/BP_Hunter.BP_Hunter_C" (Math|Transform|MakeTransform "-1710.000000,-1340.000000,88.000000") "Undefined" "MultiplyWithRoot" 0 self 0))))

(fn UpdateTime
  (Utilities|IsValid (Variables|Default|GetHUD)
    (:Is%20Valid
      (if (Variables|Default|GetbIsDone)
        (Rendering|Components|TextRender|SetText (Variables|/Game/BLUEPRINT/DUCK/WBP_HUD.WBP_HUD_C|GetTIMER (Variables|Default|GetHUD)) (Utilities|Text|ToText(Float) (Utilities|Time|GetGameTimeinSeconds) "HalfToEven"))))))