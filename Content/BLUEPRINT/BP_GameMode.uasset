(event EventBeginPlay
  (Utilities|FlowControl|Sequence
    (:then_0
      (CallFunction|CreateModeWidget))))

(event EventTick
  (params (DeltaSeconds :type Float%20%28single-precision%29))
  (switch Utilities|FlowControl|Switch|SwitchonEGameState (Variables|Default|Getstate)
    (:NewEnumerator0
      (CallFunction|WIN))
    (:NewEnumerator1
      (CallFunction|LOSE))))

(fn ConstructionScript)

(fn CreateModeWidget
  (bind _returnvalue (UserInterface|CreateWidget "/Game/BLUEPRINT/WP_GameMode.WP_GameMode_C"))
  (bind _output_get (Variables|Default|SetHUDMODE _returnvalue))
  (UserInterface|Viewport|AddtoViewport _output_get 0))

(fn WIN
  (Rendering|Components|TextRender|SetText (Variables|/Game/BLUEPRINT/WP_GameMode.WP_GameMode_C|GetTextGameState (Variables|Default|GetHUDMODE)) "YOU WIN")
  (Input|DisableInput (Game|Player|GetPlayerPawn 0) 0))

(fn UpdateState
  (params (state :type EGameState%20Enum :default "NewEnumerator0"))
  (Variables|Default|Setstate state))

(fn LOSE
  (Rendering|Components|TextRender|SetText (Variables|/Game/BLUEPRINT/WP_GameMode.WP_GameMode_C|GetTextGameState (Variables|Default|GetHUDMODE)) "YOU LOSE")
  (Input|DisableInput (Game|Player|GetPlayerPawn 0) 0))